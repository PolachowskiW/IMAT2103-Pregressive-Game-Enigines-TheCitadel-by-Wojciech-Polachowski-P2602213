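; C_Enemy is an enemy character that chases the player and deals damage on reaching them.
; BeginPlay and PawnSensing start an AI MoveTo loop that applies damage after a short delay, then chases again.
; Incoming damage lowers clamped health; death disables collision and movement, plays a random montage and destroys the actor after a delay.
; Death also updates enemy counters in the GameMode and GameInstance and shows the W_Enemies widget.
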(event `self.ReceiveBeginPlay`
  (bind _asb_character (cast `/Game/GameFiles/Blueprints/Character/B_Character` (`GameplayStatics.GetPlayerCharacter` 0)))
  (bind _output_get (set `self.CharaREF` _asb_character))
  (`self.Chase Player` _output_get))

(event `Chase Player`
  (params (Player :type "/Game/GameFiles/Blueprints/Character/B_Character Object Reference"))
  (if (not (`self.isDead?`))
    (`|AIMoveTo` self (0.0 0.0 0.0) Player
      (:`OnSuccess`
        (`KismetSystemLibrary.Delay` 0.2)
        (if (not (`self.isDead?`))
          (`GameplayStatics.ApplyDamage` Player (`self.Base Damage`))
          (`KismetSystemLibrary.Delay` 1.5)
          (`self.Chase Player` Player))))))

(event `self.PawnSensing.OnSeePawn`
  (params (Pawn :type "Pawn Object Reference"))
  (bind _asb_character (cast `/Game/GameFiles/Blueprints/Character/B_Character` Pawn))
  (`self.Chase Player` _asb_character))

(event `self.ReceiveAnyDamage`
  (params (Damage :type "Float (single-precision)") (DamageType :type "DamageType Object Reference") (InstigatedBy :type "Controller Object Reference") (DamageCauser :type "Actor Object Reference"))
  (bind _returnvalue (`self.K2_GetActorLocation`))
  (if (not (`self.isDead?`))
    (bind _output_get (set `self.Health` (`KismetMathLibrary.FClamp` (- (`self.Health`) Damage) 0.0 2.0)))
    (if (== _output_get 0.0)
      (set `self.isDead?` true)
      (`PrimitiveComponent.SetCollisionEnabled` (`self.CapsuleComponent`) "NoCollision")
      (`PrimitiveComponent.SetCollisionEnabled` (`self.Mesh`) "NoCollision")
      (`PrimitiveComponent.SetCollisionEnabled` (`self.FP_Gun`) "NoCollision")
      (`GameplayStatics.PlaySoundAtLocation` "/Game/GameFiles/SFX/Enemy_SFX/CUE_EnemyDeath.CUE_EnemyDeath" _returnvalue (struct) 1.0 1.0 0.0 null null null)
      (`|ExecutionSequence`
        (:`then_0`
          (bind _asthird_person_game_mode (cast `/Game/GameFiles/Blueprints/ThirdPersonGameMode` (`GameplayStatics.GetGameMode`)))
          (bind _result (`/Engine/EditorBlueprintResources/StandardMacros.DecrementInt` (`/Game/GameFiles/Blueprints/ThirdPersonGameMode.Enemies Left` _asthird_person_game_mode))
            (:`  `
              (set `/Game/GameFiles/Blueprints/ThirdPersonGameMode.Enemies Left` _result _asthird_person_game_mode)
              (bind _returnvalue_2 (`|CreateWidget` "/Game/GameFiles/Widgets/W_Enemies.W_Enemies_C"))
              (`UserWidget.AddToViewport` _returnvalue_2 0))))
        (:`then_1`
          (`CharacterMovementComponent.DisableMovement` (`self.CharacterMovement`))
          (`self.PlayAnimMontage` (select `int` (`KismetMathLibrary.RandomInteger` 2) :`0` "/Game/GameFiles/Animations/Death_1_Montage.Death_1_Montage" :`1` "/Game/GameFiles/Animations/Death_2_Montage.Death_2_Montage" :`2` "/Game/GameFiles/Animations/Death_3_Montage.Death_3_Montage" :!type "AnimMontage Object Reference"))
          (`KismetSystemLibrary.Delay` 40.0)
          (`self.K2_DestroyActor`))
        (:`then_2`
          (bind _asb_gi_the_citadel (cast `/Game/GameFiles/Blueprints/B_GI_TheCitadel` (`GameplayStatics.GetGameInstance`)))
          (bind _result_2 (`/Engine/EditorBlueprintResources/StandardMacros.IncrementInt` (`/Game/GameFiles/Blueprints/B_GI_TheCitadel.Enemies` _asb_gi_the_citadel))
            (:`  `
              (set `/Game/GameFiles/Blueprints/B_GI_TheCitadel.Enemies` _result_2 _asb_gi_the_citadel)))))
      (else
        (`GameplayStatics.PlaySoundAtLocation` "/Game/GameFiles/SFX/Enemy_SFX/CUE_EnemyDamage.CUE_EnemyDamage" _returnvalue (struct) 1.0 1.0 0.0 null null null)))))

(fn `UserConstructionScript`)