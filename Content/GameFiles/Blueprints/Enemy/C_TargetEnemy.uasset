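; Target enemy character that takes damage, plays hit or death sounds, and counts toward the level's target objective when killed.
; AnyDamage lowers clamped Health; at zero it decrements TargetsLeft on the game mode and increments TargetEnemies on the game instance.
; Death also disables movement and collision, plays a random death montage and destroys the actor after a delay.
; UseAmmo is empty and Reload only zeroes TempAmmo.
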(event `self.ReceiveAnyDamage`
  (params (Damage :type "Float (single-precision)") (DamageType :type "DamageType Object Reference") (InstigatedBy :type "Controller Object Reference") (DamageCauser :type "Actor Object Reference"))
  (bind _returnvalue (`self.K2_GetActorLocation`))
  (bind _output_get (set `self.Health` (`KismetMathLibrary.FClamp` (- (`self.Health`) Damage) 0.0 2.0)))
  (if (== _output_get 0.0)
    (`GameplayStatics.PlaySoundAtLocation` "/Game/GameFiles/SFX/Enemy_SFX/CUE_EnemyDeath.CUE_EnemyDeath" _returnvalue (struct) 1.0 1.0 0.0 null null null)
    (`|ExecutionSequence`
      (:`then_0`
        (bind _asthird_person_game_mode (cast `/Game/GameFiles/Blueprints/ThirdPersonGameMode` (`GameplayStatics.GetGameMode`)))
        (bind _result (`/Engine/EditorBlueprintResources/StandardMacros.DecrementInt` (`/Game/GameFiles/Blueprints/ThirdPersonGameMode.Targets Left` _asthird_person_game_mode))
          (:`  `
            (set `/Game/GameFiles/Blueprints/ThirdPersonGameMode.Targets Left` _result _asthird_person_game_mode))))
      (:`then_1`
        (`CharacterMovementComponent.DisableMovement` (`self.CharacterMovement`))
        (set `self.isDead?` true)
        (`self.PlayAnimMontage` (select `int` (`KismetMathLibrary.RandomInteger` 2) :`0` "/Game/GameFiles/Animations/Death_1_Montage.Death_1_Montage" :`1` "/Game/GameFiles/Animations/Death_2_Montage.Death_2_Montage" :`2` "/Game/GameFiles/Animations/Death_3_Montage.Death_3_Montage" :!type "AnimMontage Object Reference"))
        (`PrimitiveComponent.SetCollisionEnabled` (`self.CapsuleComponent`) "NoCollision")
        (`PrimitiveComponent.SetCollisionEnabled` (`self.Mesh`) "NoCollision")
        (`PrimitiveComponent.SetCollisionEnabled` (`self.FP_Gun`) "NoCollision")
        (`KismetSystemLibrary.Delay` 40.0)
        (`self.K2_DestroyActor`))
      (:`then_2`
        (bind _asb_gi_the_citadel (cast `/Game/GameFiles/Blueprints/B_GI_TheCitadel` (`GameplayStatics.GetGameInstance`)))
        (bind _result_2 (`/Engine/EditorBlueprintResources/StandardMacros.IncrementInt` (`/Game/GameFiles/Blueprints/B_GI_TheCitadel.Target Enemies` _asb_gi_the_citadel))
          (:`  `
            (set `/Game/GameFiles/Blueprints/B_GI_TheCitadel.Target Enemies` _result_2 _asb_gi_the_citadel)))))
    (else
      (`GameplayStatics.PlaySoundAtLocation` "/Game/GameFiles/SFX/Enemy_SFX/CUE_EnemyDamage.CUE_EnemyDamage" _returnvalue (struct) 1.0 1.0 0.0 null null null))))

(fn `Reload`
  (locals (TempAmmo :type Integer :default 0))
  (set `local.TempAmmo` 0))

(fn `Use Ammo`)

(fn `UserConstructionScript`)