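; BP_Ammo is an ammo pickup that the player collects with the Interaction input while standing inside its trigger box.
; Box overlap with B_Character enables input, shows a W_PressE prompt widget and opens a gate; leaving reverses all three.
; A press flags the widget as pressed, waits half a second, then, if the gate is open, adds ammo, plays a sound and destroys the actor.
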(event `InputAction|Interaction`
  (params (Key :type "Key Structure"))
  (:`Pressed`
    (set `/Game/GameFiles/Widgets/W_PressE.IsPressed?` true (stale `self.Box.OnComponentBeginOverlap` _returnvalue))
    (`KismetSystemLibrary.Delay` 0.5)
    (set `/Game/GameFiles/Widgets/W_PressE.IsPressed?` true (stale `self.Box.OnComponentBeginOverlap` _returnvalue))
    (`/Engine/EditorBlueprintResources/StandardMacros.Gate` true :!label _label
      (:`Exit`
        (bind _asb_character (cast `/Game/GameFiles/Blueprints/Character/B_Character` (`GameplayStatics.GetPlayerCharacter` 0)))
        (set `/Game/GameFiles/Blueprints/Character/B_Character.Ammo` (+ (`/Game/GameFiles/Blueprints/Character/B_Character.Ammo` _asb_character) 15) _asb_character)
        (`GameplayStatics.PlaySoundAtLocation` "/Game/GameFiles/SFX/mixkit-quick-win-video-game-notification-269.mixkit-quick-win-video-game-notification-269" (0.0 0.0 0.0) (struct) 0.75 1.0 0.0 null null null)
        (`self.K2_DestroyActor`)))))

(event `self.Box.OnComponentBeginOverlap`
  (params (OverlappedComponent :type "PrimitiveComponent Object Reference") (OtherActor :type "Actor Object Reference") (OtherComp :type "PrimitiveComponent Object Reference") (OtherBodyIndex :type Integer) (bFromSweep :type Boolean) (SweepResult :type "HitResult Structure (by ref)"))
  (cast `/Game/GameFiles/Blueprints/Character/B_Character` OtherActor)
  (`self.EnableInput` (`GameplayStatics.GetPlayerController` 0))
  (bind _returnvalue (`|CreateWidget` "/Game/GameFiles/Widgets/W_PressE.W_PressE_C"))
  (`UserWidget.AddToViewport` _returnvalue 0)
  (goto _label :!via `Open`))

(event `self.Box.OnComponentEndOverlap`
  (params (OverlappedComponent :type "PrimitiveComponent Object Reference") (OtherActor :type "Actor Object Reference") (OtherComp :type "PrimitiveComponent Object Reference") (OtherBodyIndex :type Integer))
  (cast `/Game/GameFiles/Blueprints/Character/B_Character` OtherActor)
  (`self.DisableInput` (`GameplayStatics.GetPlayerController` 0))
  (`Widget.RemoveFromParent` (stale `self.Box.OnComponentBeginOverlap` _returnvalue))
  (goto _label :!via `Close`))

(fn `UserConstructionScript`)