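; BP_Bullet is a gun projectile that resolves on its first hit.
; Actors tagged Target, Enemy or Friendly take a small fixed damage, with the bullet as damage causer.
; Every hit destroys the bullet and spawns a muzzle flash particle attached to Sphere1 as the impact effect.
; For untagged hits, the effect spawns after the destroy call instead of before it.
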(event `self.ReceiveHit`
  (params (MyComp :type "PrimitiveComponent Object Reference") (Other :type "Actor Object Reference") (OtherComp :type "PrimitiveComponent Object Reference") (bSelfMoved :type Boolean) (HitLocation :type "Vector Structure") (HitNormal :type "Vector Structure") (NormalImpulse :type "Vector Structure") (Hit :type "HitResult Structure (by ref)"))
  (if (or (`self.ActorHasTag` Other "Target") (`self.ActorHasTag` Other "Enemy") (`self.ActorHasTag` Other "Friendly"))
    (`GameplayStatics.ApplyDamage` Other 1.0 null self)
    (`GameplayStatics.SpawnEmitterAttached` "/Game/InfinityBladeEffects/Effects/FX_Monsters/FX_Monster_Chicken/P_ChickenMaster_MuzzleFlash_01.P_ChickenMaster_MuzzleFlash_01" (`self.Sphere1`) "None" (0.0 0.0 0.0) (struct :`Yaw` 180.0))
    (`self.K2_DestroyActor`)
    (else
      (`self.K2_DestroyActor`)
      (`GameplayStatics.SpawnEmitterAttached` "/Game/InfinityBladeEffects/Effects/FX_Monsters/FX_Monster_Chicken/P_ChickenMaster_MuzzleFlash_01.P_ChickenMaster_MuzzleFlash_01" (`self.Sphere1`) "None" (0.0 0.0 0.0) (struct :`Yaw` 180.0)))))

(fn `UserConstructionScript`)