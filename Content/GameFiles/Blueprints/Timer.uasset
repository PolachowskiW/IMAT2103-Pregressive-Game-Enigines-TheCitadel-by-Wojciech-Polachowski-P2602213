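; Countdown timer actor that ends the game in a Game Over when minutes and seconds run out.
; Tick feeds a one-second Delay that plays an alarm beep and decrements the clock while the player is alive and has not won.
; At zero it shows the Game Over widget and cursor and pauses the game, with a switch to the character's death camera queued behind a short Delay.
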(event `self.ReceiveTick`
  (params (DeltaSeconds :type "Float (single-precision)"))
  (bind _asb_character (cast `/Game/GameFiles/Blueprints/Character/B_Character` (`GameplayStatics.GetPlayerCharacter` 0)))
  (bind _asthird_person_game_mode (cast `/Game/GameFiles/Blueprints/ThirdPersonGameMode` (`GameplayStatics.GetGameMode`)))
  (if (not (`/Game/GameFiles/Blueprints/Character/B_Character.isDead?` _asb_character))
    (if (not (`/Game/GameFiles/Blueprints/ThirdPersonGameMode.win` _asthird_person_game_mode))
      (`KismetSystemLibrary.Delay` 1.0)
      (bind _output_get (set `self.volume` (`self.volume`)))
      (`GameplayStatics.PlaySoundAtLocation` "/Game/GameFiles/SFX/mixkit-alarm-clock-beep-988.mixkit-alarm-clock-beep-988" (0.0 0.0 0.0) (struct) _output_get 1.0 0.0 null null null)
      (if (== (`self.Seconds`) 0)
        (if (== (`self.Minutes`) 0)
          (`|ExecutionSequence`
            (:`then_0`
              (`KismetSystemLibrary.Delay` 0.5)
              (bind _asb_character_2 (cast `/Game/GameFiles/Blueprints/Character/B_Character` (`GameplayStatics.GetPlayerCharacter` 0)))
              (`ActorComponent.SetActive` (`/Game/GameFiles/Blueprints/Character/B_Character.DeathCamera` _asb_character_2) true false)
              (`ActorComponent.SetActive` (`/Game/GameFiles/Blueprints/Character/B_Character.Aim Camera` _asb_character_2) false false)
              (`ActorComponent.SetActive` (`/Game/GameFiles/Blueprints/Character/B_Character.DeathCamera1` _asb_character_2) false false)
              (`ActorComponent.SetActive` (`/Game/GameFiles/Blueprints/Character/B_Character.PlayerCamera` _asb_character_2) false false))
            (:`then_1`
              (bind _returnvalue (`|CreateWidget` "/Game/GameFiles/Widgets/W_Game_Over.W_Game_Over_C"))
              (`UserWidget.AddToViewport` _returnvalue 0)
              (set `PlayerController.bShowMouseCursor` true (`GameplayStatics.GetPlayerController` 0))
              (`GameplayStatics.SetGamePaused` true)))
          (else
            (set `self.Seconds` 59)
            (set `self.Minutes` (- (`self.Minutes`) 1))))
        (else
          (set `self.Seconds` (- (`self.Seconds`) 1)))))))

(fn `UserConstructionScript`)